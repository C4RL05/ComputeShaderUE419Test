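; Test actor that exercises compute shader calculations from Blueprint, going by its name.
; On BeginPlay it initializes two input positions and two scalars, then calls CalculateYZUpdated with fixed XYZ values if both initializations succeed.
; Releasing key 1 or 2 re-seeds the scalars with random whole-number floats, then runs Calculate or CalculateYZUpdated respectively.
; The calculation functions are not defined in this graph, and their results are not read here.
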(event EventBeginPlay
  (bind _returnvalue (Class|TestComputeShaderActor|InitializeInputPositions (Utilities|Array|MakeArray "1.000000,2.000000,3.000000" "4.000000,5.000000,6.000000")))
  (if _returnvalue
    (bind _returnvalue_2 (Class|TestComputeShaderActor|InitializeInputScalars (Utilities|Array|MakeArray 3.0 0.5)))
    (if _returnvalue_2
      (Class|TestComputeShaderActor|CalculateYZUpdated 5.0 4.0 3.0))))

(event Input|KeyboardEvents|1
  (params (Key :type Key%20Structure))
  (:Released
    (bind _returnvalue (Class|TestComputeShaderActor|InitializeInputScalars (Utilities|Array|MakeArray (Math|Conversions|ToFloat(Integer) (Math|Random|RandomIntegerinRange -3 5)) (Math|Conversions|ToFloat(Integer) (Math|Random|RandomIntegerinRange -3 5)))))
    (if _returnvalue
      (Class|TestComputeShaderActor|Calculate 5.0))))

(event Input|KeyboardEvents|2
  (params (Key :type Key%20Structure))
  (:Released
    (bind _returnvalue (Class|TestComputeShaderActor|InitializeInputScalars (Utilities|Array|MakeArray (Math|Conversions|ToFloat(Integer) (Math|Random|RandomIntegerinRange -3 5)) (Math|Conversions|ToFloat(Integer) (Math|Random|RandomIntegerinRange -3 5)))))
    (if _returnvalue
      (Class|TestComputeShaderActor|CalculateYZUpdated 5.0 4.0 3.0))))

(fn ConstructionScript)